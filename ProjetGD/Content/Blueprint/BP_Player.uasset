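; Player character Blueprint that handles first-hand movement, look and jump input through legacy axis and action mappings.
; Look axes feed controller yaw and pitch, while the move axes add movement input along the forward and right vectors of the full control rotation, pitch included.
; The jump action calls Jump on press, BeginPlay only prints a debug message, and Tick, overlap and the construction script are empty.
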(event EventBeginPlay
  (Development|PrintText "Hey Bitch !"))

(event EventActorBeginOverlap
  (params (OtherActor :type Actor%20Object%20Reference)))

(event EventTick
  (params (DeltaSeconds :type Float%20%28single-precision%29)))

(event Input|ActionEvents|InputActionjump_action
  (params (Key :type Key%20Structure :default "AnyKey"))
  (:Pressed
    (Character|Jump)))

(event Input|AxisEvents|InputAxisforward_axis
  (params (AxisValue :type Float%20%28single-precision%29))
  ;[1 1 1] Translate
  (Pawn|Input|AddMovementInput (Math|Vector|GetForwardVector (Pawn|GetControlRotation :!class /Script/Engine.Pawn)) AxisValue false))

(event Input|AxisEvents|InputAxisright_axis
  (params (AxisValue :type Float%20%28single-precision%29))
  ;[1 1 1] Translate
  (Pawn|Input|AddMovementInput (Math|Vector|GetRightVector (Pawn|GetControlRotation :!class /Script/Engine.Pawn)) AxisValue false))

(event Input|AxisEvents|InputAxisrotate_up_down
  (params (AxisValue :type Float%20%28single-precision%29))
  ;[1 1 1] Rotate
  (Pawn|Input|AddControllerPitchInput AxisValue))

(event Input|AxisEvents|InputAxisrotate_left_right
  (params (AxisValue :type Float%20%28single-precision%29))
  ;[1 1 1] Rotate
  (Pawn|Input|AddControllerYawInput AxisValue))

(fn ConstructionScript)